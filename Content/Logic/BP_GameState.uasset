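; Game state Blueprint that presents the end-of-game screen and the restart animation.
; GameFinished waits briefly on a win, then shows UW_Finish with the result and the first player's points from PAC_PlayerState, and enables the mouse cursor.
; ShowResetAnimation plays the LS_Restart level sequence through a player created on demand, whose actor is destroyed when playback finishes.
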(event `self.GameFinished`
  (params (win :type Boolean))
  (bind _returnvalue (`GameplayStatics.GetPlayerController` 0))
  (if win
    (`KismetSystemLibrary.Delay` 1.5))
  (bind _aspac_player_state (cast `PAC_PlayerState` (`Controller.PlayerState` _returnvalue)))
  (bind _returnvalue_2 (`|CreateWidget` "/Game/Logic/UI/UW_Finish.UW_Finish_C" _returnvalue win (`PAC_PlayerState.CurrentPoints` _aspac_player_state)))
  (`UserWidget.AddToViewport` _returnvalue_2 999)
  (set `PlayerController.bShowMouseCursor` true (`GameplayStatics.GetPlayerController` 0)))

(event `self.ShowResetAnimation`
  (bind (_outactor _returnvalue) (`LevelSequencePlayer.CreateLevelSequencePlayer` "/Game/Levels/MainLevel/LS_Restart.LS_Restart"))
  (add `MovieSceneSequencePlayer.OnFinished` _returnvalue (delegate `OnFinished_Event_0`))
  (`MovieSceneSequencePlayer.Play` _returnvalue))

(event `OnFinished_Event_0`
  (`self.K2_DestroyActor` (stale `self.ShowResetAnimation` _outactor)))

(fn `UserConstructionScript`)